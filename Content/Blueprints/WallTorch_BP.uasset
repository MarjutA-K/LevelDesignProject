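; WallTorch_BP is a wall torch prop with a fire sound.
; Its construction script assigns meshes from three variables to the Torch component and two other static mesh components.
; On BeginPlay it starts the Fire01Cue audio from the beginning; the overlap and tick events are unused.
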(event `self.ReceiveBeginPlay`
  (`AudioComponent.Play` (`self.Fire01_Cue`) 0.0))

(fn `UserConstructionScript`
  (`StaticMeshComponent.SetStaticMesh` (`self.Torch`) (`self.New Mesh`))
  (`StaticMeshComponent.SetStaticMesh` (`self.StaticMesh`) (`self.New Mesh_0`))
  (`StaticMeshComponent.SetStaticMesh` (`self.StaticMesh1`) (`self.New Mesh_1`)))