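; Quest item pickup that the player collects by pressing Q while inside its Box trigger.
; SetVisibilityOn applies the item's visibility setting and briefly shows a pickup widget.
; Box overlap toggles actor input and, for the ThirdPersonCharacter, a Gate that lets Q through.
; Collecting adds the key part amount to the character's QuestItem, destroys the actor, plays an enemies-approaching sound and shakes the camera.
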(event `SetVisibilityOn`
  (`SceneComponent.SetVisibility` (`self.QuestItem`) (`self.Quest Item Visibility`) false)
  (bind _returnvalue (`|CreateWidget` "/Game/Widgets/PickUp_Widget.PickUp_Widget_C"))
  (`UserWidget.AddToViewport` _returnvalue 0)
  (`KismetSystemLibrary.Delay` 2.0)
  (`Widget.RemoveFromParent` _returnvalue)
  (`self.EnableInput` (`GameplayStatics.GetPlayerController` 0) :!label _label)
  (cast `/Game/ThirdPersonBP/Blueprints/ThirdPersonCharacter` (stale `self.Box.OnComponentBeginOverlap` OtherActor))
  (goto _label_2 :!via `Open`))

(event `Key|Q`
  (params (Key :type "Key Structure"))
  (:`Pressed`
    (`/Engine/EditorBlueprintResources/StandardMacros.Gate` true :!label _label_2
      (:`Exit`
        (bind _asthird_person_character (cast `/Game/ThirdPersonBP/Blueprints/ThirdPersonCharacter` (`GameplayStatics.GetPlayerCharacter` 0)))
        (set `/Game/ThirdPersonBP/Blueprints/ThirdPersonCharacter.QuestItem` (+ (`/Game/ThirdPersonBP/Blueprints/ThirdPersonCharacter.QuestItem` _asthird_person_character) (`self.KeyPart_Single`)) _asthird_person_character)
        (`self.K2_DestroyActor`)
        (`GameplayStatics.PlaySound2D` "/Game/StarterContent/Audio/MediumEnemiesApproaching_Cue.MediumEnemiesApproaching_Cue" 1.0 1.0 0.0 null null)
        (bind _followcamera (`/Game/ThirdPersonBP/Blueprints/ThirdPersonCharacter.FollowCamera` _asthird_person_character))
        (`CameraComponent.GetCameraView` _followcamera 0.0)
        (`GameplayStatics.PlayWorldCameraShake` "/Game/Blueprints/CameraShake1.CameraShake1_C" (`SceneComponent.K2_GetComponentLocation` _followcamera) 100.0 1000.0)))))

(event `self.Box.OnComponentBeginOverlap`
  (params (OverlappedComponent :type "PrimitiveComponent Object Reference") (OtherActor :type "Actor Object Reference") (OtherComp :type "PrimitiveComponent Object Reference") (OtherBodyIndex :type Integer) (bFromSweep :type Boolean) (SweepResult :type "HitResult Structure (by ref)"))
  (goto _label))

(event `self.Box.OnComponentEndOverlap`
  (params (OverlappedComponent :type "PrimitiveComponent Object Reference") (OtherActor :type "Actor Object Reference") (OtherComp :type "PrimitiveComponent Object Reference") (OtherBodyIndex :type Integer))
  (`self.DisableInput` (`GameplayStatics.GetPlayerController` 0))
  (cast `/Game/ThirdPersonBP/Blueprints/ThirdPersonCharacter` OtherActor)
  (goto _label_2 :!via `Close`))

(fn `UserConstructionScript`)