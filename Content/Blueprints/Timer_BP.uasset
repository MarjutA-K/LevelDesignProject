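; Timer actor that counts down Minutes and Seconds and shows a YouDied widget when time has run out.
; When the ThirdPersonCharacter begins overlapping its Box, it waits one second, then decrements Seconds, rolling over into Minutes at zero.
; Each overlap event drives at most one step with no loop, and the widget appears only if both values are already zero at that step.
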(event `self.ReceiveTick`
  (params (DeltaSeconds :type "Float (single-precision)")))

(event `self.Box.OnComponentBeginOverlap`
  (params (OverlappedComponent :type "PrimitiveComponent Object Reference") (OtherActor :type "Actor Object Reference") (OtherComp :type "PrimitiveComponent Object Reference") (OtherBodyIndex :type Integer) (bFromSweep :type Boolean) (SweepResult :type "HitResult Structure (by ref)"))
  (cast `/Game/ThirdPersonBP/Blueprints/ThirdPersonCharacter` OtherActor)
  (`KismetSystemLibrary.Delay` 1.0)
  (if (== (`self.Seconds`) 0)
    (if (== (`self.Minutes`) 0)
      (bind _returnvalue (`|CreateWidget` "/Game/Widgets/YouDied_Widget.YouDied_Widget_C"))
      (`UserWidget.AddToViewport` _returnvalue 0)
      (else
        (set `self.Seconds` 59)
        (set `self.Minutes` (- (`self.Minutes`) 1))))
    (else
      (set `self.Seconds` (- (`self.Seconds`) 1)))))

(fn `UserConstructionScript`)