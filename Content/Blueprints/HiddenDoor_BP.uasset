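; Hidden door actor that opens when a ThirdPersonCharacter holding enough quest items enters its trigger box.
; Box overlap compares the character's QuestItem to QuestItemRequiredAmount, then plays the OpenDoor timeline, which drives the Door's relative location.
; When the character leaves the box, the timeline reverses without rechecking the item count.
; The construction script applies the Scale variable to the Door's world scale.
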(event `self.Box.OnComponentBeginOverlap`
  (params (OverlappedComponent :type "PrimitiveComponent Object Reference") (OtherActor :type "Actor Object Reference") (OtherComp :type "PrimitiveComponent Object Reference") (OtherBodyIndex :type Integer) (bFromSweep :type Boolean) (SweepResult :type "HitResult Structure (by ref)"))
  (bind _asthird_person_character (cast `/Game/ThirdPersonBP/Blueprints/ThirdPersonCharacter` OtherActor))
  (if (>= (`/Game/ThirdPersonBP/Blueprints/ThirdPersonCharacter.QuestItem` _asthird_person_character) (`self.QuestItemRequiredAmount`))
    (bind (_direction _newtrack_0) (`Timeline|Open door` :!label _label)
      (:`Update`
        (`SceneComponent.K2_SetRelativeLocation` (`self.Door`) _newtrack_0 false false)))))

(event `self.Box.OnComponentEndOverlap`
  (params (OverlappedComponent :type "PrimitiveComponent Object Reference") (OtherActor :type "Actor Object Reference") (OtherComp :type "PrimitiveComponent Object Reference") (OtherBodyIndex :type Integer))
  (cast `/Game/ThirdPersonBP/Blueprints/ThirdPersonCharacter` OtherActor)
  (goto _label :!via `Reverse`))

(fn `UserConstructionScript`
  (`SceneComponent.SetWorldScale3D` (`self.Door`) (`self.Scale`)))