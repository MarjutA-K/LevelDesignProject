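; A respawning pickup actor that flies toward the player and reappears at its start point after collection.
; Entering the Range trigger plays a timeline that interpolates the actor toward player character 0 each update, adding a vector track offset.
; Touching the PickUp trigger sets Collected and hides the actor, then a five-second timer moves it back to its saved location, unhides it and clears the flag.
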(event `self.ReceiveBeginPlay`
  (set `self.start_point` (`self.K2_GetActorLocation`)))

(event `self.Range.OnComponentBeginOverlap`
  (params (OverlappedComponent :type "PrimitiveComponent Object Reference") (OtherActor :type "Actor Object Reference") (OtherComp :type "PrimitiveComponent Object Reference") (OtherBodyIndex :type Integer) (bFromSweep :type Boolean) (SweepResult :type "HitResult Structure (by ref)"))
  (if (== OtherActor (`GameplayStatics.GetPlayerCharacter` 0))
    (if (not (`self.collected`))
      (bind (_direction _newtrack_2) (`Timeline|Timeline_0` :!via `PlayFromStart`)
        (:`Update`
          (`self.K2_SetActorLocation` (+ _newtrack_2 (`KismetMathLibrary.VInterpTo` (.location (`self.GetTransform`)) (`self.K2_GetActorLocation` (`GameplayStatics.GetPlayerCharacter` 0)) (`GameplayStatics.GetWorldDeltaSeconds`) 15.0))))))))

(event `self.PickUp.OnComponentBeginOverlap`
  (params (OverlappedComponent :type "PrimitiveComponent Object Reference") (OtherActor :type "Actor Object Reference") (OtherComp :type "PrimitiveComponent Object Reference") (OtherBodyIndex :type Integer) (bFromSweep :type Boolean) (SweepResult :type "HitResult Structure (by ref)"))
  (if (== OtherActor (`GameplayStatics.GetPlayerCharacter` 0))
    (set `self.collected` true)
    (`self.SetActorHiddenInGame` true)
    (`KismetSystemLibrary.K2_SetTimerDelegate` (delegate `Respawn`) 5.0)))

(event `Respawn`
  (`self.K2_SetActorLocation` (`self.start_point`))
  (`self.SetActorHiddenInGame` false)
  (set `self.collected` false))

(fn `UserConstructionScript`)