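; Elevator actor whose platform travels to an end position while a mesh component overlaps its trigger Box, and returns when an overlap ends.
; Overlap events play or reverse the MovePlatform timeline at a rate of 1/Duration, lerping StartPlatform from its BeginPlay location to EndPlatformLocation.
; The construction script applies the shared mesh, scale and rotation to both platforms and places EndPlatform at the destination.
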(event `self.ReceiveBeginPlay`
  (set `self.StartLocation` (`SceneComponent.RelativeLocation` (`self.StartPlatform`))))

(event `self.Box.OnComponentBeginOverlap`
  (params (OverlappedComponent :type "PrimitiveComponent Object Reference") (OtherActor :type "Actor Object Reference") (OtherComp :type "PrimitiveComponent Object Reference") (OtherBodyIndex :type Integer) (bFromSweep :type Boolean) (SweepResult :type "HitResult Structure (by ref)"))
  (cast `MeshComponent` OtherComp)
  (`TimelineComponent.SetPlayRate` (`self.move platform`) (/ 1.0 (`self.Duration`)))
  (bind (_direction _move_track) (`Timeline|move platform` :!label _label)
    (:`Update`
      (`SceneComponent.K2_SetRelativeLocation` (`self.StartPlatform`) (`KismetMathLibrary.VLerp` (`self.StartLocation`) (`self.EndPlatform Location`) _move_track) false false))))

(event `self.Box.OnComponentEndOverlap`
  (params (OverlappedComponent :type "PrimitiveComponent Object Reference") (OtherActor :type "Actor Object Reference") (OtherComp :type "PrimitiveComponent Object Reference") (OtherBodyIndex :type Integer))
  (cast `MeshComponent` OtherComp)
  (`TimelineComponent.SetPlayRate` (`self.move platform`) (/ 1.0 (`self.Duration`)))
  (goto _label :!via `Reverse`))

(fn `UserConstructionScript`
  (bind _startplatform (`self.StartPlatform`))
  (bind _endplatform (`self.EndPlatform`))
  (bind _platformmesh (`self.PlatformMesh`))
  (`StaticMeshComponent.SetStaticMesh` _startplatform _platformmesh)
  (`StaticMeshComponent.SetStaticMesh` _endplatform _platformmesh)
  (`SceneComponent.SetRelativeScale3D` _startplatform (`self.Scale`))
  (`SceneComponent.SetRelativeScale3D` _endplatform (`self.Scale`))
  (`SceneComponent.K2_SetRelativeRotation` _endplatform (`self.Rotation`) false false)
  (`SceneComponent.K2_SetRelativeRotation` _startplatform (`self.Rotation`) false false)
  (`SceneComponent.K2_SetRelativeLocation` _endplatform (`self.EndPlatform Location`) false false))