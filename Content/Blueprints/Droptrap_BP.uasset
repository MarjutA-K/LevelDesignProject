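; Droptrap_BP is a trap that drops a referenced Trap actor when the player's ThirdPersonCharacter overlaps its Trigger.
; BeginPlay caches the player and the trap's start location, sets the timeline rate from Speed, and zeroes the delay unless HasDelay is set.
; After that delay, TrapTimeLine lerps the trap's Z to TrapFallLocation without sweeping.
; A fixed delay chained from the timeline's Update then reverses it, returning the trap.
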(event `self.ReceiveBeginPlay`
  (bind _asthird_person_character (cast `/Game/ThirdPersonBP/Blueprints/ThirdPersonCharacter` (`GameplayStatics.GetPlayerPawn` 0))
    (:`then`
      (set `self.PlayerRef` _asthird_person_character)
      (set `self.TrapLocation` (`SceneComponent.K2_GetComponentLocation` (`Actor.RootComponent` (`self.Trap`))))
      (`TimelineComponent.SetPlayRate` (`self.TrapTimeLine`) (`self.Speed`))
      (if (`self.HasDelay`)
        (set `self.Delay` (`self.Delay`))
        (else
          (set `self.Delay` 0.0))))
    (:`CastFailed`
      (`KismetSystemLibrary.PrintString` "Failed to cast"))))

(event `self.Trigger.OnComponentBeginOverlap`
  (params (OverlappedComponent :type "PrimitiveComponent Object Reference") (OtherActor :type "Actor Object Reference") (OtherComp :type "PrimitiveComponent Object Reference") (OtherBodyIndex :type Integer) (bFromSweep :type Boolean) (SweepResult :type "HitResult Structure (by ref)"))
  (bind _traplocation (`self.TrapLocation`))
  (`KismetSystemLibrary.Delay` (`self.Delay`))
  (if (== OtherActor (`self.PlayerRef`))
    (bind (_direction _trapmovement) (`Timeline|TrapTimeLine` :!label _label)
      (:`Update`
        (`self.K2_SetActorLocation` (`self.Trap`) (`KismetMathLibrary.VLerp` _traplocation (`KismetMathLibrary.MakeVector` (.x _traplocation) (.y _traplocation) (`self.TrapFallLocation`)) _trapmovement) false false)
        (`KismetSystemLibrary.Delay` 7.0)
        (goto _label :!via `Reverse`)))))

(fn `UserConstructionScript`)