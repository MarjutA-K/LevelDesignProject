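; A one-shot trigger actor that plays the CutSceneCredits level sequence when the player character overlaps its Box.
; The sequence player is created on BeginPlay, and the overlap disables the player's input and starts playback.
; A timer matched to the sequence's duration then re-enables input and destroys the trigger.
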(event `self.ReceiveBeginPlay`
  (bind (_outactor _returnvalue) (`LevelSequencePlayer.CreateLevelSequencePlayer` "/Game/CutScenes/CutSceneCredits.CutSceneCredits"))
  (set `self.CutScene` _returnvalue))

(event `self.Box.OnComponentBeginOverlap`
  (params (OverlappedComponent :type "PrimitiveComponent Object Reference") (OtherActor :type "Actor Object Reference") (OtherComp :type "PrimitiveComponent Object Reference") (OtherBodyIndex :type Integer) (bFromSweep :type Boolean) (SweepResult :type "HitResult Structure (by ref)"))
  (bind _returnvalue (`GameplayStatics.GetPlayerCharacter` 0))
  (bind _cutscene (`self.CutScene`))
  (if (== OtherActor _returnvalue)
    (`self.DisableInput` _returnvalue (`GameplayStatics.GetPlayerController` 0))
    (`MovieSceneSequencePlayer.Play` _cutscene)
    (`KismetSystemLibrary.K2_SetTimerDelegate` (delegate `enable movement`) (`TimeManagementBlueprintLibrary.Conv_QualifiedFrameTimeToSeconds` (`MovieSceneSequencePlayer.GetDuration` _cutscene)))))

(event `enable movement`
  (`self.EnableInput` (`GameplayStatics.GetPlayerCharacter` 0) (`GameplayStatics.GetPlayerController` 0))
  (`self.K2_DestroyActor`))

(fn `UserConstructionScript`)