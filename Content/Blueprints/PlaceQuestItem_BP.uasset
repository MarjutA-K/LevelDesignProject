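; Quest item placement spot that triggers the ending credits and returns to the main menu.
; Box overlap enables input, briefly shows a put-down prompt, then stops the audio started at BeginPlay.
; Q reveals the item and, if the overlapping actor is the player, disables player input and plays the credits sequence, music and widget.
; A timer matching the sequence length fires EnableMovement, which, despite its name, opens MainMenuLevel.
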(event `self.ReceiveBeginPlay`
  (`AudioComponent.Play` (`self.Audio`) 0.0)
  (bind (_outactor _returnvalue) (`LevelSequencePlayer.CreateLevelSequencePlayer` "/Game/CutScenes/CutSceneCredits.CutSceneCredits"))
  (set `self.CutScene` _returnvalue))

(event `self.Box.OnComponentBeginOverlap`
  (params (OverlappedComponent :type "PrimitiveComponent Object Reference") (OtherActor :type "Actor Object Reference") (OtherComp :type "PrimitiveComponent Object Reference") (OtherBodyIndex :type Integer) (bFromSweep :type Boolean) (SweepResult :type "HitResult Structure (by ref)"))
  (`self.EnableInput` (`GameplayStatics.GetPlayerController` 0))
  (bind _returnvalue (`|CreateWidget` "/Game/Widgets/PutDown_Widget.PutDown_Widget_C"))
  (`UserWidget.AddToViewport` _returnvalue 0)
  (`KismetSystemLibrary.Delay` 2.0)
  (`Widget.RemoveFromParent` _returnvalue)
  (`AudioComponent.Stop` (`self.Audio`)))

(event `Key|Q`
  (params (Key :type "Key Structure"))
  (bind _returnvalue (`GameplayStatics.GetPlayerCharacter` 0))
  (bind _cutscene (`self.CutScene`))
  (:`Pressed`
    (`SceneComponent.SetVisibility` (`self.QuestItem`) true false)
    (`KismetSystemLibrary.Delay` 0.5)
    (if (== (stale `self.Box.OnComponentBeginOverlap` OtherActor) _returnvalue)
      (`self.DisableInput` _returnvalue (`GameplayStatics.GetPlayerController` 0))
      (`MovieSceneSequencePlayer.Play` _cutscene)
      (`KismetSystemLibrary.K2_SetTimerDelegate` (delegate `enable movement`) (`TimeManagementBlueprintLibrary.Conv_QualifiedFrameTimeToSeconds` (`MovieSceneSequencePlayer.GetDuration` _cutscene)))
      (`GameplayStatics.PlaySound2D` "/Game/StarterContent/Audio/CreditMusic__Cue.CreditMusic__Cue" 1.0 1.0 0.0 null null)
      (`WidgetLayoutLibrary.RemoveAllWidgets`)
      (bind _returnvalue_2 (`|CreateWidget` "/Game/Widgets/CreditWidget.CreditWidget_C"))
      (`UserWidget.AddToViewport` _returnvalue_2 0))))

(event `enable movement`
  (`GameplayStatics.OpenLevel` "MainMenuLevel"))

(fn `UserConstructionScript`)