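; Spike wall hazard actor that moves back and forth and damages actors that overlap it.
; On BeginPlay a timeline starts and drives the Spikewall component's relative location.
; The timeline's Update pin, rather than Finished, also feeds a Delay, after which a Loop flag alternates between reversing and playing the timeline.
; Any actor overlap sends a small fixed damage amount through TakeDamageMessage to the other actor.
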(event `self.ReceiveBeginPlay`
  (bind (_direction _newtrack_0) (`Timeline|Timeline_0` :!label _label)
    (:`Update`
      (`SceneComponent.K2_SetRelativeLocation` (`self.Spikewall`) _newtrack_0 false false)
      (`KismetSystemLibrary.Delay` (`self.Duration`))
      (if (`self.Loop`)
        (set `self.Loop` false)
        (goto _label :!via `Reverse`)
        (else
          (set `self.Loop` true)
          (goto _label))))))

(event `self.ReceiveActorBeginOverlap`
  (params (OtherActor :type "Actor Object Reference"))
  (message `/Game/Blueprints/Damageable_BP.Take Damage` OtherActor 0.1))

(fn `UserConstructionScript`)